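; BP_Battle_Manager sets up and resolves autobattler combat between the player and an opponent.
; StartBattle caches placements from the player camera and Opponent, then InitOpponent clears and refills the opponent's placements with new, uninitialized BP_Items.
; BattleRound, not called here, uses per-side counters to pick the next player creature and a random opponent creature, then calls AttackTarget.
; The Attack function is an unfinished stub with disconnected logic.
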(event `StartBattle`
  (`|ExecutionSequence`
    (:`then_0`
      (bind _asbp_player_camera (cast `/Game/AutobattlerProject/Blueprint/Core/BP_PlayerCamera` (`GameplayStatics.GetPlayerPawn` 0)))
      (set `self.PlacementsPlayer_0` (`/Game/AutobattlerProject/Blueprint/Core/BP_PlayerCamera.PlayerPlacement` _asbp_player_camera)))
    (:`then_1`
      (set `self.PlacementsPlayer_1` (`/Game/AutobattlerProject/Blueprint/Core/TestOpponent.Placements` (`self.Opponent`))))
    (:`then_2`
      (`self.Init Opponent`))))

(fn `Attack`
  (params (From :type "/Game/AutobattlerProject/Blueprint/Gameplay/BoardGameObjects/Product/BP_Creature Object Reference") (To :type "/Game/AutobattlerProject/Blueprint/Gameplay/BoardGameObjects/Product/BP_Creature Object Reference"))
  (locals (L_Attack :type Integer) (L_Health :type Integer)))

(fn `Battle Round`
  (locals (L_AttackingCreature :type "/Game/AutobattlerProject/Blueprint/Gameplay/BoardGameObjects/Product/BP_Creature Object Reference") (L_AttackedCreature :type "/Game/AutobattlerProject/Blueprint/Gameplay/BoardGameObjects/Product/BP_Creature Object Reference"))
  (bind _placement (`self.SearchPlacementAttackedCreature`))
  (bind _placement_2 (`self.SearchPlacementAttackingCreature`))
  (`|ExecutionSequence`
    (:`then_0`
      (`/Engine/EditorBlueprintResources/StandardMacros.IsValid` _placement_2
        (:`Is Valid`
          (bind (_bisvalid _boardgameobject) (message `/Game/AutobattlerProject/Blueprint/Interface/BPI_Placement.Get Object From Placement` _placement_2))
          (bind _asbp_creature (cast `/Game/AutobattlerProject/Blueprint/Gameplay/BoardGameObjects/Product/BP_Creature` _boardgameobject))
          (set `local.L_AttackingCreature` _asbp_creature))))
    (:`then_1`
      (`/Engine/EditorBlueprintResources/StandardMacros.IsValid` _placement
        (:`Is Valid`
          (bind (_bisvalid_2 _boardgameobject_2) (message `/Game/AutobattlerProject/Blueprint/Interface/BPI_Placement.Get Object From Placement` _placement))
          (bind _asbp_creature_2 (cast `/Game/AutobattlerProject/Blueprint/Gameplay/BoardGameObjects/Product/BP_Creature` _boardgameobject_2))
          (set `local.L_AttackedCreature` _asbp_creature_2))))
    (:`then_2`
      (`/Game/AutobattlerProject/Blueprint/Gameplay/BoardGameObjects/Product/BP_Creature.AttackTarget` (`local.L_AttackingCreature`) (`local.L_AttackedCreature`)))))

(fn `Init Opponent`
  (bind _keys (`BlueprintMapLibrary.Map_Keys` (`/Game/AutobattlerProject/Blueprint/Core/TestOpponent.CreatureMap` (`self.Opponent`))))
  (for _array_element _keys
    (`|ExecutionSequence`
      (:`then_0`
        (`/Game/AutobattlerProject/Blueprint/Gameplay/BoardGameObjects/Placement/BP_Placement_Base.ClearPlacement` _array_element))
      (:`then_1`
        (`/Engine/EditorBlueprintResources/StandardMacros.IsValid` (`BlueprintMapLibrary.Map_Find` (`/Game/AutobattlerProject/Blueprint/Core/TestOpponent.CreatureMap` (`self.Opponent`)) _array_element)
          (:`Is Valid`
            (bind _returnvalue (`|GenericCreateObject` "/Game/AutobattlerProject/Blueprint/Gameplay/BoardGameObjects/BP_Item.BP_Item_C" self))
            (`/Game/AutobattlerProject/Blueprint/Gameplay/BoardGameObjects/Placement/BP_Placement_Base.Try Create Object in Placement` _array_element _returnvalue)))))))

(fn `SearchPlacementAttackedCreature`
  (returns (Placement :type "/Game/AutobattlerProject/Blueprint/Gameplay/BoardGameObjects/Placement/BP_Placement_Base Object Reference"))
  (locals (L_Placement :type "/Game/AutobattlerProject/Blueprint/Gameplay/BoardGameObjects/Placement/BP_Placement_Base Object Reference") (L_PotentialTarget :type "Array of /Game/AutobattlerProject/Blueprint/Gameplay/BoardGameObjects/Placement/BP_Placement_Base Object Reference"))
  (for (_array_element _array_index) (`self.PlacementsPlayer_1`)
    (set `local.L_Placement` _array_element)
    (if (>= _array_index (`self.Count_Player_1`))
      (`/Engine/EditorBlueprintResources/StandardMacros.IncrementInt` (`self.Count_Player_1`)
        (:`  `
          (bind _bisvalid (message `/Game/AutobattlerProject/Blueprint/Interface/BPI_Placement.Get Object From Placement` (`local.L_Placement`)))
          (if _bisvalid
            (`KismetArrayLibrary.Array_Add` (`local.L_PotentialTarget`) (`local.L_Placement`)))))))
  (return (`KismetArrayLibrary.Array_Random` (`local.L_PotentialTarget`))))

(fn `SearchPlacementAttackingCreature`
  (returns (Placement :type "/Game/AutobattlerProject/Blueprint/Gameplay/BoardGameObjects/Placement/BP_Placement_Base Object Reference"))
  (locals (L_Placement :type "/Game/AutobattlerProject/Blueprint/Gameplay/BoardGameObjects/Placement/BP_Placement_Base Object Reference") (L_Count :type Integer :default 0))
  (for (_array_element _array_index) (`self.PlacementsPlayer_0`)
    (set `local.L_Placement` _array_element)
    (if (>= _array_index (`self.Count_Player_0`))
      (`/Engine/EditorBlueprintResources/StandardMacros.IncrementInt` (`self.Count_Player_0`)
        (:`  `
          (bind _bisvalid (message `/Game/AutobattlerProject/Blueprint/Interface/BPI_Placement.Get Object From Placement` (`local.L_Placement`)))
          (if _bisvalid
            (return (`local.L_Placement`))))))))

(fn `UserConstructionScript`)