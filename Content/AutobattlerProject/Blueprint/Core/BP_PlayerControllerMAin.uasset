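; Main player controller for the autobattler: creates the HUD and relays pointer input and card plays to the event manager.
; Each tick it broadcasts the world point under the mouse, or first touch on mobile, found by line trace.
; A card-play event spawns a board object at the card's traced screen position, injects a drag interaction strategy, then fires interact-start and card-play events.
; Battle manager init is empty; actor and area detection are unwired.
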(event `self.ReceiveBeginPlay`
  (`|ExecutionSequence`
    (:`then_0`
      (`self.InitHUD`))
    (:`then_1`
      (`self.InitEvents`))
    (:`then_2`
      (`self.Init BattleManager`))))

(event `Key|LeftMouseButton`
  (params (Key :type "Key Structure"))
  (:`Pressed`
    (`/Game/AutobattlerProject/Blueprint/Core/BP_EventManager.OnInteractStart` (`/Game/AutobattlerProject/Blueprint/FunctionLibraries/BPFL_Events.Get Event Manager`)))
  (:`Released`
    (`/Game/AutobattlerProject/Blueprint/Core/BP_EventManager.OnInteractEnd` (`/Game/AutobattlerProject/Blueprint/FunctionLibraries/BPFL_Events.Get Event Manager`))))

(event `OnCardPlayStart_Event`
  (params (Card :type "Object Object Reference") (CardScreenPosition :type "Vector2D Structure"))
  (bind _item (message `/Game/AutobattlerProject/Blueprint/Interface/BPI_Item.GetItem` Card))
  (bind _newgameobject (`self.Create Game Object at Location` (`self.Get Location by Screen Position` CardScreenPosition) _item))
  (`/Game/AutobattlerProject/Blueprint/Core/BP_EventManager.OnInteractStart` (`/Game/AutobattlerProject/Blueprint/FunctionLibraries/BPFL_Events.Get Event Manager`))
  (`/Game/AutobattlerProject/Blueprint/Core/BP_EventManager.OnCardPlay` (`/Game/AutobattlerProject/Blueprint/FunctionLibraries/BPFL_Events.Get Event Manager`) _newgameobject _item))

(event `self.ReceiveTick`
  (params (DeltaSeconds :type "Float (single-precision)"))
  (set `self.Mouse Location` (`self.Mouse Location to World Space`))
  (`/Game/AutobattlerProject/Blueprint/Core/BP_EventManager.OnMouseLocationUpdate` (`/Game/AutobattlerProject/Blueprint/FunctionLibraries/BPFL_Events.Get Event Manager`) (`self.Mouse Location`)))

(fn `AreaDetected`
  (returns (AreaActor :type "Actor Object Reference"))
  (locals (WorldLocation :type "Vector Structure") (WorldDirection :type "Vector Structure"))
  (bind (_locationx _locationy) (`self.GetInputTouchState` "Touch1"))
  (bind (_worldlocation _worlddirection) (`self.DeprojectMousePositionToWorld`))
  (bind _worldlocation_2 (`local.WorldLocation`))
  (bind (_worldposition _worlddirection_2) (`GameplayStatics.DeprojectScreenToWorld` null (`KismetMathLibrary.MakeVector2D` _locationx _locationy)))
  (if (`self.bIsMobile`)
    (set `local.WorldLocation` _worldposition) ; Mobile World Location
    (set `local.WorldDirection` _worlddirection_2) ; Moble World Direction
    (else
      (set `local.WorldLocation` _worldlocation)
      (set `local.WorldDirection` _worlddirection)))
  (bind _outhit (`KismetSystemLibrary.LineTraceSingleForObjects` :`Start` _worldlocation_2 :`End` (+ _worldlocation_2 (* (`local.WorldDirection`) 1000.0)) :`ObjectTypes` (`|MakeArray` "ObjectTypeQuery8" :!type "EObjectTypeQuery Enum") :`DrawTime` 10.0))
  (return (`.HitActor` (`GameplayStatics.BreakHitResult` _outhit))))

(fn `Create Game Object at Location`
  (params (Location :type "Vector Structure") (Item :type "/Game/AutobattlerProject/Blueprint/Gameplay/BoardGameObjects/BP_Item Object Reference"))
  (returns (NewGameObject :type "/Game/AutobattlerProject/Blueprint/Gameplay/BoardGameObjects/BoardGameObjects/BP_BoardGameObjectsBase Object Reference"))
  (bind _returnvalue (`|SpawnActorFromClass` "/Game/AutobattlerProject/Blueprint/Gameplay/BoardGameObjects/BoardGameObjects/BP_BoardGameObjectsBase.BP_BoardGameObjectsBase_C" (`KismetMathLibrary.MakeTransform` (`KismetMathLibrary.MakeVector` (.x Location) (.y Location) 20.0)) "Undefined" "OverrideRootScale" null Item (`GameplayStatics.GetPlayerPawn` 0)))
  (bind _returnvalue_2 (`|GenericCreateObject` "/Game/AutobattlerProject/Blueprint/Gameplay/BoardGameObjects/BoardGameObjects/Interact/BP_Interact_DragObject.BP_Interact_DragObject_C" _returnvalue _returnvalue (`/Game/AutobattlerProject/Blueprint/FunctionLibraries/BPFL_Events.Get Event Manager`)))
  (message `/Game/AutobattlerProject/Blueprint/Interface/BPI_BoardObject.Set Interact Strategy` _returnvalue _returnvalue_2)
  (return _returnvalue))

(fn `Get Location by Screen Position`
  (params (`Screen Position` :type "Vector2D Structure"))
  (returns (Location :type "Vector Structure"))
  (bind (_worldposition _worlddirection) (`GameplayStatics.DeprojectScreenToWorld` self `Screen Position`))
  (bind _outhit (`KismetSystemLibrary.LineTraceSingleForObjects` :`Start` _worldposition :`End` (+ _worldposition (* _worlddirection (`self.TraceDistance`))) :`ObjectTypes` (`|MakeArray` "ObjectTypeQuery1" :!type "EObjectTypeQuery Enum") :`DrawTime` 10.0))
  (return (`.Location` (`GameplayStatics.BreakHitResult` _outhit))))

(fn `Init BattleManager`)

(fn `InitEvents`
  (`|ExecutionSequence`
    (:`then_0`
      (add `/Game/AutobattlerProject/Blueprint/Core/BP_EventManager.OnCardPlayStart` (`/Game/AutobattlerProject/Blueprint/FunctionLibraries/BPFL_Events.Get Event Manager`) (`|CreateDelegate` :!event `OnCardPlayStart_Event`)))))

(fn `InitHUD`
  (bind _returnvalue (`|CreateWidget` "/Game/AutobattlerProject/UI/WBP_HUD.WBP_HUD_C"))
  (bind _output_get (set `self.WBP_HUD` _returnvalue))
  (`UserWidget.AddToViewport` _output_get 0))

(fn `InteractedActorDetected`
  (params (IgnoredActor :type "Actor Object Reference"))
  (returns (HitActor :type "Actor Object Reference"))
  (locals (WorldLocation :type "Vector Structure") (WorldDirection :type "Vector Structure"))
  (bind (_locationx _locationy) (`self.GetInputTouchState` "Touch1"))
  (bind (_worldlocation _worlddirection) (`self.DeprojectMousePositionToWorld`))
  (bind _worldlocation_2 (`local.WorldLocation`))
  (bind (_worldposition _worlddirection_2) (`GameplayStatics.DeprojectScreenToWorld` null (`KismetMathLibrary.MakeVector2D` _locationx _locationy)))
  (if (`self.bIsMobile`)
    (set `local.WorldLocation` _worldposition) ; Mobile World Location
    (set `local.WorldDirection` _worlddirection_2) ; Moble World Direction
    (else
      (set `local.WorldLocation` _worldlocation)
      (set `local.WorldDirection` _worlddirection)))
  (bind _outhit (`KismetSystemLibrary.LineTraceSingleForObjects` _worldlocation_2 (+ _worldlocation_2 (* (`local.WorldDirection`) (`self.TraceDistance`))) (`|MakeArray` "ObjectTypeQuery9" :!type "EObjectTypeQuery Enum") false (`|MakeArray` IgnoredActor) "None" true (struct :`R` 1.0 :`A` 1.0) (struct :`G` 1.0 :`A` 1.0) 10.0))
  (return (`.HitActor` (`GameplayStatics.BreakHitResult` _outhit))))

(fn `Mouse Distance in World Space`
  (returns (Location :type "Vector Structure") (`Spawn Tranfrom` :type "Transform Structure"))
  (bind (_worldlocation _worlddirection) (`self.DeprojectMousePositionToWorld`))
  (bind _returnvalue (+ _worldlocation (* _worlddirection (`self.TraceDistance`))))
  (return _returnvalue (`KismetMathLibrary.MakeTransform` _returnvalue)))

(fn `Mouse Location to World Space`
  (returns (Location :type "Vector Structure"))
  (locals (WorldLocation :type "Vector Structure") (WorldDirection :type "Vector Structure"))
  (bind (_locationx _locationy) (`self.GetInputTouchState` "Touch1"))
  (bind (_worldlocation _worlddirection) (`self.DeprojectMousePositionToWorld`))
  (bind _worldlocation_2 (`local.WorldLocation`))
  (bind (_worldposition _worlddirection_2) (`GameplayStatics.DeprojectScreenToWorld` null (`KismetMathLibrary.MakeVector2D` _locationx _locationy)))
  (if (`self.bIsMobile`)
    (set `local.WorldLocation` _worldposition) ; Mobile World Location
    (set `local.WorldDirection` _worlddirection_2) ; Moble World Direction
    (else
      (set `local.WorldLocation` _worldlocation)
      (set `local.WorldDirection` _worlddirection)))
  (bind _outhit (`KismetSystemLibrary.LineTraceSingleForObjects` :`Start` _worldlocation_2 :`End` (+ _worldlocation_2 (* (`local.WorldDirection`) (`self.TraceDistance`))) :`ObjectTypes` (`|MakeArray` "ObjectTypeQuery1" :!type "EObjectTypeQuery Enum") :`DrawTime` 10.0))
  (return (`.Location` (`GameplayStatics.BreakHitResult` _outhit))))

(fn `UserConstructionScript`)