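; BP_FieldManager tracks the board placements of both sides in the autobattler and snapshots the player's side.
; On BeginPlay, InitField gathers every PlacementBase actor and sorts it into player or opponent lists by the IsPlayer flag in its config, exposed through getters.
; ArchivingField stores the item from each occupied player placement in SaveItems, keyed by placement index; no restore logic is present here.
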(event `self.ReceiveBeginPlay`
  (`self.InitField`))

(fn `ArchivingField`
  (locals (LSaveItems :type "Map of Integer to /Game/AutobattlerProject/Gameplay/BoardGameObjects/BP_Item Object Reference"))
  (for _array_element (`self.PlayerPlacement`)
    (bind (_bisvalid _boardgameobject) (message `/Game/AutobattlerProject/Interface/BPI_Placement.Get Object From Placement` _array_element))
    (if _bisvalid
      (bind _item (message `/Game/AutobattlerProject/Interface/BPI_ItemInfo.GetItem` _boardgameobject))
      (bind _placementinfo (message `/Game/AutobattlerProject/Interface/BPI_ObjectInteract.GetPlacementConfig` _array_element))
      (`BlueprintMapLibrary.Map_Add` (`local.LSaveItems`) (`.Index` (break `OBSPlacementInfo` _placementinfo)) _item)))
  (set `self.SaveItems` (`local.LSaveItems`)))

(fn `GetOpponentPlacement`
  (returns (OpponentPlacement :type "Array of PlacementBase Object Reference"))
  (return (`self.OpponentPlacement`)))

(fn `GetPlayerPlacement`
  (returns (PlayerPlacement :type "Array of PlacementBase Object Reference"))
  (locals (LPlayerPlacement :type "Array of PlacementBase Object Reference"))
  (return (`self.PlayerPlacement`)))

(fn `InitField`
  (locals (LPlacement :type "PlacementBase Object Reference"))
  (bind _outactors (`GameplayStatics.GetAllActorsOfClass` "/Script/AutobattlerProject.PlacementBase"))
  (bind _output_get (set `self.AllPlacement` _outactors))
  (for _array_element _output_get
    (bind _output_get_2 (set `local.LPlacement` _array_element))
    (bind _placementinfo (message `/Game/AutobattlerProject/Interface/BPI_ObjectInteract.GetPlacementConfig` _output_get_2))
    (if (`.bIsPlayer` (break `OBSPlacementInfo` _placementinfo))
      (`KismetArrayLibrary.Array_Add` (`self.PlayerPlacement`) (`local.LPlacement`))
      (else
        (`KismetArrayLibrary.Array_Add` (`self.OpponentPlacement`) (`local.LPlacement`))))))

(fn `UserConstructionScript`)