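; Main player controller for the autobattler that creates the HUD and relays mouse input to the Event Manager.
; Left and right button presses and releases become manager events, and every Tick broadcasts the cursor's world location.
; That location comes from a deprojected line trace against WorldStatic objects, using Touch1 on mobile and the mouse otherwise.
; Battle manager and event initialization are empty stubs.
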(event `self.ReceiveBeginPlay`
  (`|ExecutionSequence`
    (:`then_0`
      (`self.InitHUD`))
    (:`then_1`
      (`self.InitEvents`))
    (:`then_2`
      (`self.Init BattleManager`))))

(event `Key|LeftMouseButton`
  (params (Key :type "Key Structure"))
  (:`Pressed`
    (`/Game/AutobattlerProject/Blueprint/Events/BP_EventManager.OnLMBPressed` (`/Game/AutobattlerProject/Blueprint/FunctionLibraries/BPFL_Events.Get Event Manager`)))
  (:`Released`
    (`/Game/AutobattlerProject/Blueprint/Events/BP_EventManager.OnLMBReleased` (`/Game/AutobattlerProject/Blueprint/FunctionLibraries/BPFL_Events.Get Event Manager`))))

(event `Key|RightMouseButton`
  (params (Key :type "Key Structure"))
  (:`Pressed`
    (`/Game/AutobattlerProject/Blueprint/Events/BP_EventManager.OnRMBPressed` (`/Game/AutobattlerProject/Blueprint/FunctionLibraries/BPFL_Events.Get Event Manager`)))
  (:`Released`
    (`/Game/AutobattlerProject/Blueprint/Events/BP_EventManager.OnRMBReleased` (`/Game/AutobattlerProject/Blueprint/FunctionLibraries/BPFL_Events.Get Event Manager`))))

(event `self.ReceiveTick`
  (params (DeltaSeconds :type "Float (single-precision)"))
  (set `self.Mouse Location` (`self.Mouse Location to World Space`))
  (`/Game/AutobattlerProject/Blueprint/Events/BP_EventManager.OnMouseLocationUpdate` (`/Game/AutobattlerProject/Blueprint/FunctionLibraries/BPFL_Events.Get Event Manager`) (`self.Mouse Location`)))

(fn `Get Location by Screen Position`
  (params (`Screen Position` :type "Vector2D Structure"))
  (returns (Location :type "Vector Structure"))
  (bind (_worldposition _worlddirection) (`GameplayStatics.DeprojectScreenToWorld` self `Screen Position`))
  (bind _outhit (`KismetSystemLibrary.LineTraceSingleForObjects` :`Start` _worldposition :`End` (+ _worldposition (* _worlddirection (`self.TraceDistance`))) :`ObjectTypes` (`|MakeArray` "ObjectTypeQuery1" :!type "EObjectTypeQuery Enum") :`DrawTime` 10.0))
  (return (`.Location` (`GameplayStatics.BreakHitResult` _outhit))))

(fn `Init BattleManager`)

(fn `InitEvents`
  (`|ExecutionSequence`))

(fn `InitHUD`
  (bind _returnvalue (`|CreateWidget` "/Game/AutobattlerProject/UI/WBP_HUD.WBP_HUD_C"))
  (bind _output_get (set `self.WBP_HUD` _returnvalue))
  (`UserWidget.AddToViewport` _output_get 0))

(fn `Mouse Distance in World Space`
  (returns (Location :type "Vector Structure") (`Spawn Tranfrom` :type "Transform Structure"))
  (bind (_worldlocation _worlddirection) (`self.DeprojectMousePositionToWorld`))
  (bind _returnvalue (+ _worldlocation (* _worlddirection (`self.TraceDistance`))))
  (return _returnvalue (`KismetMathLibrary.MakeTransform` _returnvalue)))

(fn `Mouse Location to World Space`
  (returns (Location :type "Vector Structure"))
  (locals (WorldLocation :type "Vector Structure") (WorldDirection :type "Vector Structure"))
  (bind (_locationx _locationy) (`self.GetInputTouchState` "Touch1"))
  (bind (_worldlocation _worlddirection) (`self.DeprojectMousePositionToWorld`))
  (bind _worldlocation_2 (`local.WorldLocation`))
  (bind (_worldposition _worlddirection_2) (`GameplayStatics.DeprojectScreenToWorld` null (`KismetMathLibrary.MakeVector2D` _locationx _locationy)))
  (if (`self.bIsMobile`)
    (set `local.WorldLocation` _worldposition) ; Mobile World Location
    (set `local.WorldDirection` _worlddirection_2) ; Moble World Direction
    (else
      (set `local.WorldLocation` _worldlocation)
      (set `local.WorldDirection` _worlddirection)))
  (bind _outhit (`KismetSystemLibrary.LineTraceSingleForObjects` :`Start` _worldlocation_2 :`End` (+ _worldlocation_2 (* (`local.WorldDirection`) (`self.TraceDistance`))) :`ObjectTypes` (`|MakeArray` "ObjectTypeQuery1" :!type "EObjectTypeQuery Enum") :`DrawTime` 10.0))
  (return (`.Location` (`GameplayStatics.BreakHitResult` _outhit))))

(fn `UserConstructionScript`)