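; Player controller for the autobattler that connects the HUD to the shop and battle manager and handles dragging actors between areas.
; On BeginPlay it creates the HUD, finds the store and battle manager, and binds their HUD events.
; Left mouse press and release use mouse or touch object traces to grab an actor and move it to the detected area through messages.
; PlayCard is empty, and older buy, sell and card-placement logic is disconnected.
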(event `self.ReceiveBeginPlay`
  (`|ExecutionSequence`
    (:`then_0`
      (`self.InitHUD`))
    (:`then_1`
      (`self.Init Shop`))
    (:`then_2`
      (`self.Init BattleManager`))))

(event `Key|LeftMouseButton`
  (params (Key :type "Key Structure"))
  (:`Pressed`
    (bind (_location _hitactor) (`self.Mouse To World Space` (`self.InteractActor`)))
    (set `self.InteractActor` _hitactor)
    (set `self.PastArea` (`self.AreaDetected`))
    (message `/Game/AutobattlerProject/Blueprint/Interface/BPI_ObjectInteract.StartInteract` (`self.InteractActor`)))
  (:`Released`
    (bind _interactactor (`self.InteractActor`)
      (:`then`
        (message `/Game/AutobattlerProject/Blueprint/Interface/BPI_AreaInteract.MoveToArea` (`self.AreaDetected`) (`self.PastArea`) _interactactor)
        (message `/Game/AutobattlerProject/Blueprint/Interface/BPI_ObjectInteract.EndInteract` (`self.InteractActor`))
        (set `self.InteractActor` null)
        (set `self.InteractActor` null))
      (:`else`))))

(event `PlayCard`
  (params (`Card Info` :type "/Game/AutobattlerProject/Blueprint/Struct/FPlayingCardInfo Structure")))

(fn `AreaDetected`
  (returns (AreaActor :type "Actor Object Reference"))
  (locals (WorldLocation :type "Vector Structure") (WorldDirection :type "Vector Structure"))
  (bind (_locationx _locationy) (`self.GetInputTouchState` "Touch1"))
  (bind (_worldlocation _worlddirection) (`self.DeprojectMousePositionToWorld`))
  (bind _worldlocation_2 (`local.WorldLocation`))
  (bind (_worldposition _worlddirection_2) (`GameplayStatics.DeprojectScreenToWorld` null (`KismetMathLibrary.MakeVector2D` _locationx _locationy)))
  (if (`self.bIsMobile`)
    (set `local.WorldLocation` _worldposition) ; Mobile World Location
    (set `local.WorldDirection` _worlddirection_2) ; Moble World Direction
    (else
      (set `local.WorldLocation` _worldlocation)
      (set `local.WorldDirection` _worlddirection)))
  (bind _outhit (`KismetSystemLibrary.LineTraceSingleForObjects` :`Start` _worldlocation_2 :`End` (+ _worldlocation_2 (* (`local.WorldDirection`) 1000.0)) :`ObjectTypes` (`|MakeArray` "ObjectTypeQuery8" :!type "EObjectTypeQuery Enum") :`DrawTime` 10.0))
  (return (`.HitActor` (`GameplayStatics.BreakHitResult` _outhit))))

(fn `Get Actor Under Widget`
  (params (`Screen Position` :type "Vector2D Structure"))
  (returns (bIsActortFound :type Boolean) (HitActor :type "Actor Object Reference") (bIsStore :type Boolean))
  (bind (_x _y) (`KismetMathLibrary.BreakVector2D` `Screen Position`))
  (bind (_worldposition _worlddirection) (`GameplayStatics.DeprojectScreenToWorld` self (`KismetMathLibrary.MakeVector2D` _x _y)))
  (bind (_outhit _returnvalue) (`KismetSystemLibrary.LineTraceSingleForObjects` :`Start` _worldposition :`End` (+ _worldposition (* _worlddirection (`self.TraceDistance`))) :`ObjectTypes` (`|MakeArray` "ObjectTypeQuery9" "ObjectTypeQuery8" :!type "EObjectTypeQuery Enum") :`DrawTime` 10.0))
  (bind (_bblockinghit _binitialoverlap _time _distance _location _impactpoint _normal _impactnormal _physmat _hitactor) (`GameplayStatics.BreakHitResult` _outhit))
  (return _returnvalue _hitactor (`.bSuccess` (cast `/Game/AutobattlerProject/Blueprint/Gameplay/BoardGameObjects/GameArea/BP_StoreArea` _hitactor :!pure true))))

(fn `Init BattleManager`
  (bind _outactors (`GameplayStatics.GetAllActorsOfClass` "/Game/AutobattlerProject/Blueprint/Core/BP_Battle_Manager.BP_Battle_Manager_C"))
  (bind _output_get (set `self.BattleManager` (`|GetArrayItem` _outactors)))
  (add `/Game/AutobattlerProject/UI/WBP_HUD.OnStartBattle` (`self.WBP_HUD`) (`|CreateDelegate` _output_get :!event `StartBattle`))
  (add `/Game/AutobattlerProject/UI/WBP_HUD.OnNextRound` (`self.WBP_HUD`) (`|CreateDelegate` (`self.BattleManager`) :!event `Battle Round`)))

(fn `Init Shop`
  (bind _outactors (`GameplayStatics.GetAllActorsOfClass` "/Game/AutobattlerProject/Blueprint/Gameplay/BoardGameObjects/GameArea/BP_Store.BP_Store_C"))
  (bind _output_get (set `self.ShopManager` (`|GetArrayItem` _outactors)))
  (add `/Game/AutobattlerProject/UI/WBP_HUD.OnLevelUpShop` (`self.WBP_HUD`) (`|CreateDelegate` _output_get :!event `ShopLevelUp`))
  (add `/Game/AutobattlerProject/UI/WBP_HUD.OnRefreshShop` (`self.WBP_HUD`) (`|CreateDelegate` (`self.ShopManager`) :!event `ShopRefresh`)))

(fn `InitHUD`
  (bind _returnvalue (`|CreateWidget` "/Game/AutobattlerProject/UI/WBP_HUD.WBP_HUD_C"))
  (bind _output_get (set `self.WBP_HUD` _returnvalue))
  (add `/Game/AutobattlerProject/UI/WBP_HUD.OnPlayCard` _output_get (`|CreateDelegate` :!event `PlayCard`))
  (`UserWidget.AddToViewport` _output_get 0))

(fn `Mouse Distance in World Space`
  (returns (Location :type "Vector Structure") (`Spawn Tranfrom` :type "Transform Structure"))
  (bind (_worldlocation _worlddirection) (`self.DeprojectMousePositionToWorld`))
  (bind _returnvalue (+ _worldlocation (* _worlddirection (`self.TraceDistance`))))
  (return _returnvalue (`KismetMathLibrary.MakeTransform` _returnvalue)))

(fn `Mouse To World Space`
  (params (IgnoredActor :type "Actor Object Reference"))
  (returns (Location :type "Vector Structure") (HitActor :type "Actor Object Reference"))
  (locals (WorldLocation :type "Vector Structure") (WorldDirection :type "Vector Structure"))
  (bind (_locationx _locationy) (`self.GetInputTouchState` "Touch1"))
  (bind (_worldlocation _worlddirection) (`self.DeprojectMousePositionToWorld`))
  (bind _worldlocation_2 (`local.WorldLocation`))
  (bind (_worldposition _worlddirection_2) (`GameplayStatics.DeprojectScreenToWorld` null (`KismetMathLibrary.MakeVector2D` _locationx _locationy)))
  (if (`self.bIsMobile`)
    (set `local.WorldLocation` _worldposition) ; Mobile World Location
    (set `local.WorldDirection` _worlddirection_2) ; Moble World Direction
    (else
      (set `local.WorldLocation` _worldlocation)
      (set `local.WorldDirection` _worlddirection)))
  (bind _outhit (`KismetSystemLibrary.LineTraceSingleForObjects` _worldlocation_2 (+ _worldlocation_2 (* (`local.WorldDirection`) (`self.TraceDistance`))) (`|MakeArray` "ObjectTypeQuery1" "ObjectTypeQuery9" :!type "EObjectTypeQuery Enum") false (`|MakeArray` IgnoredActor) "None" true (struct :`R` 1.0 :`A` 1.0) (struct :`G` 1.0 :`A` 1.0) 10.0))
  (bind (_bblockinghit _binitialoverlap _time _distance _location _impactpoint _normal _impactnormal _physmat _hitactor) (`GameplayStatics.BreakHitResult` _outhit))
  (return _location _hitactor))

(fn `UserConstructionScript`)