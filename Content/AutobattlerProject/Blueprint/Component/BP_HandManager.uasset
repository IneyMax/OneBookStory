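; BP_HandManager is a hand manager component for card add and remove events in the autobattler project.
; On BeginPlay it binds to the event manager's card-added-to-hand and card-removed-from-hand events, whose handlers here are still empty.
; A separate InitHUD function creates WBP_HUD, stores it and adds it to the viewport, but nothing in this Blueprint calls it.
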(event `self.ReceiveBeginPlay`
  (`self.InitEvents`))

(event `OnCardAddToHand_Event`
  (params (AddedGameObject :type "Actor Object Reference") (Item :type "Object Object Reference")))

(event `OnCardRemoveFromHand_Event`
  (params (CreatedGameObject :type "Actor Object Reference") (Item :type "Object Object Reference")))

(fn `InitEvents`
  (`|ExecutionSequence`
    (:`then_0`
      (add `/Game/AutobattlerProject/Blueprint/Core/BP_EventManager.OnCardAddToHand` (`/Game/AutobattlerProject/Blueprint/FunctionLibraries/BPFL_Events.Get Event Manager`) (`|CreateDelegate` :!event `OnCardAddToHand_Event`)))
    (:`then_1`
      (add `/Game/AutobattlerProject/Blueprint/Core/BP_EventManager.OnCardRemoveFromHand` (`/Game/AutobattlerProject/Blueprint/FunctionLibraries/BPFL_Events.Get Event Manager`) (`|CreateDelegate` :!event `OnCardRemoveFromHand_Event`)))))

(fn `InitHUD`
  (bind _returnvalue (`|CreateWidget` "/Game/AutobattlerProject/UI/WBP_HUD.WBP_HUD_C"))
  (bind _output_get (set `self.WBP_HUD` _returnvalue))
  (`UserWidget.AddToViewport` _output_get 0))