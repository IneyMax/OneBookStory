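; BP_ItemsComponent is an autobattler component that translates item buy, sell, play and return-to-hand events into hand and board updates.
; On BeginPlay it binds handlers to those four events on the event manager.
; Each handler re-broadcasts two lower-level events through the same manager, passing the game object and item along.
; Buy and return add to hand, play adds to board, and sell removes from both.
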(event `self.ReceiveBeginPlay`
  (`self.InitEvents`))

(event `OnGameObjectBuy_Event`
  (params (PurchasedGameObject :type "Actor Object Reference") (Item :type "Object Object Reference"))
  (`/Game/AutobattlerProject/Blueprint/Core/BP_EventManager.OnCardAddToHand` (`/Game/AutobattlerProject/Blueprint/FunctionLibraries/BPFL_Events.Get Event Manager`) PurchasedGameObject Item)
  (`/Game/AutobattlerProject/Blueprint/Core/BP_EventManager.OnGameObjectRemoveFromBoard` (`/Game/AutobattlerProject/Blueprint/FunctionLibraries/BPFL_Events.Get Event Manager`) PurchasedGameObject Item))

(event `OnGameObjectSell_Event`
  (params (SoldGameObject :type "Actor Object Reference") (Item :type "Object Object Reference"))
  (`/Game/AutobattlerProject/Blueprint/Core/BP_EventManager.OnCardRemoveFromHand` (`/Game/AutobattlerProject/Blueprint/FunctionLibraries/BPFL_Events.Get Event Manager`) SoldGameObject Item)
  (`/Game/AutobattlerProject/Blueprint/Core/BP_EventManager.OnGameObjectRemoveFromBoard` (`/Game/AutobattlerProject/Blueprint/FunctionLibraries/BPFL_Events.Get Event Manager`) SoldGameObject Item))

(event `OnCardPlayed_Event`
  (params (CreatedGameObject :type "Actor Object Reference") (Item :type "Object Object Reference"))
  (`/Game/AutobattlerProject/Blueprint/Core/BP_EventManager.OnGameObjectAddToBoard` (`/Game/AutobattlerProject/Blueprint/FunctionLibraries/BPFL_Events.Get Event Manager`) CreatedGameObject Item)
  (`/Game/AutobattlerProject/Blueprint/Core/BP_EventManager.OnCardRemoveFromHand` (`/Game/AutobattlerProject/Blueprint/FunctionLibraries/BPFL_Events.Get Event Manager`) CreatedGameObject Item))

(event `OnGameObjectReturnToHand_Event`
  (params (GameObject :type "Actor Object Reference") (Item :type "Object Object Reference"))
  (`/Game/AutobattlerProject/Blueprint/Core/BP_EventManager.OnCardAddToHand` (`/Game/AutobattlerProject/Blueprint/FunctionLibraries/BPFL_Events.Get Event Manager`) GameObject Item)
  (`/Game/AutobattlerProject/Blueprint/Core/BP_EventManager.OnGameObjectRemoveFromBoard` (`/Game/AutobattlerProject/Blueprint/FunctionLibraries/BPFL_Events.Get Event Manager`) GameObject Item))

(fn `InitEvents`
  (`|ExecutionSequence`
    (:`then_0`
      (add `/Game/AutobattlerProject/Blueprint/Core/BP_EventManager.OnGameObjectBuy` (`/Game/AutobattlerProject/Blueprint/FunctionLibraries/BPFL_Events.Get Event Manager`) (`|CreateDelegate` :!event `OnGameObjectBuy_Event`)))
    (:`then_1`
      (add `/Game/AutobattlerProject/Blueprint/Core/BP_EventManager.OnGameObjectSell` (`/Game/AutobattlerProject/Blueprint/FunctionLibraries/BPFL_Events.Get Event Manager`) (`|CreateDelegate` :!event `OnGameObjectSell_Event`)))
    (:`then_2`
      (add `/Game/AutobattlerProject/Blueprint/Core/BP_EventManager.OnCardPlayed` (`/Game/AutobattlerProject/Blueprint/FunctionLibraries/BPFL_Events.Get Event Manager`) (`|CreateDelegate` :!event `OnCardPlayed_Event`)))
    (:`then_3`
      (add `/Game/AutobattlerProject/Blueprint/Core/BP_EventManager.OnGameObjectReturnToHand` (`/Game/AutobattlerProject/Blueprint/FunctionLibraries/BPFL_Events.Get Event Manager`) (`|CreateDelegate` :!event `OnGameObjectReturnToHand_Event`)))))