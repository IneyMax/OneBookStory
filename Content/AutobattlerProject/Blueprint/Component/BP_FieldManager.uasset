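; BP_FieldManager is a Blueprint component in the autobattler project that reacts to game objects entering and leaving the board.
; On BeginPlay it binds to the event manager's add-to-board and remove-from-board events, and also calls an unbind from card-play-cancel.
; The removal handler calls RemoveFromBoardMessage on the affected object, while the add handler is empty.
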(event `self.ReceiveBeginPlay`
  (`self.InitEvents`))

(event `OnGameObjectAddToBoard_Event`
  (params (GameObjectAdded :type "Actor Object Reference") (Item :type "Object Object Reference")))

(event `OnGameObjectRemoveFromBoard_Event`
  (params (GameObject :type "Actor Object Reference") (Item :type "Object Object Reference"))
  (message `/Game/AutobattlerProject/Blueprint/Interface/BPI_BoardObject.RemoveFromBoard` GameObject))

(fn `InitEvents`
  (`|ExecutionSequence`
    (:`then_0`
      (add `/Game/AutobattlerProject/Blueprint/Core/BP_EventManager.OnGameObjectAddToBoard` (`/Game/AutobattlerProject/Blueprint/FunctionLibraries/BPFL_Events.Get Event Manager`) (`|CreateDelegate` :!event `OnGameObjectAddToBoard_Event`)))
    (:`then_1`
      (add `/Game/AutobattlerProject/Blueprint/Core/BP_EventManager.OnGameObjectRemoveFromBoard` (`/Game/AutobattlerProject/Blueprint/FunctionLibraries/BPFL_Events.Get Event Manager`) (`|CreateDelegate` :!event `OnGameObjectRemoveFromBoard_Event`)))
    (:`then_2`
      (remove `/Game/AutobattlerProject/Blueprint/Core/BP_EventManager.OnCardPlayCancel` (`/Game/AutobattlerProject/Blueprint/FunctionLibraries/BPFL_Events.Get Event Manager`) (`|CreateDelegate` :!event `OnGameObjectRemoveFromBoard_Event`)))))