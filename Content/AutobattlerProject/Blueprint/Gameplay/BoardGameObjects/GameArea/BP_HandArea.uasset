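; BP_HandArea is the board area representing the player's hand in the autobattler.
; When an actor moves into it, it reads the actor's item message and notifies the event manager based on the source area.
; Arrivals from the store raise a buy event, while arrivals from the player field raise a move-to-hand event.
; The construction script scales its collision box from CollisionScale.
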(event `/Game/AutobattlerProject/Blueprint/Interface/BPI_AreaInteract.MoveToArea`
  (params (PastArea :type "Actor Object Reference") (MovedActor :type "Actor Object Reference"))
  (cast `/Game/AutobattlerProject/Blueprint/Gameplay/BoardGameObjects/GameArea/BP_StoreArea` PastArea
    (:`then`
      (bind _item (message `/Game/AutobattlerProject/Blueprint/Interface/BPI_Item.GetItem` MovedActor))
      (`/Game/AutobattlerProject/Blueprint/Core/BP_EventManager.OnBuy` (`/Game/AutobattlerProject/Blueprint/FunctionLibraries/BPFL_Events.Get Event Manager`) MovedActor _item))
    (:`CastFailed`
      (cast `/Game/AutobattlerProject/Blueprint/Gameplay/BoardGameObjects/GameArea/BP_PlayerFieldArea` PastArea)
      (bind _item_2 (message `/Game/AutobattlerProject/Blueprint/Interface/BPI_Item.GetItem` MovedActor))
      (`/Game/AutobattlerProject/Blueprint/Core/BP_EventManager.OnMoveGameObjectToHand` (`/Game/AutobattlerProject/Blueprint/FunctionLibraries/BPFL_Events.Get Event Manager`) MovedActor _item_2))))

(fn `UserConstructionScript`
  (`SceneComponent.SetRelativeScale3D` (`self.Box`) (`self.CollisionScale`)))