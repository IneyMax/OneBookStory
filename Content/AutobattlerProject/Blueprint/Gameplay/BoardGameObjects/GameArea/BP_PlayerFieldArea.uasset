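; BP_PlayerFieldArea is a board area, apparently the player's field, that accepts objects moved onto it in the autobattler.
; MoveToArea rejects moves from itself and accepts all others, firing the event manager's game object purchase event with the object's item message when it comes from a BP_StoreArea.
; The construction script scales its box to CollisionScale, and GetItem is left empty.
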(fn `GetItem`
  (returns (Item :type "/Game/AutobattlerProject/Blueprint/Gameplay/BoardGameObjects/BP_Item Object Reference"))
  (return null))

(fn `MoveToArea`
  (params (PastArea :type "Actor Object Reference") (MovedActor :type "Actor Object Reference"))
  (returns (bIsAreaChange :type Boolean))
  (if (!= PastArea self)
    (cast `/Game/AutobattlerProject/Blueprint/Gameplay/BoardGameObjects/GameArea/BP_StoreArea` PastArea
      (:`then`
        (bind _item (message `/Game/AutobattlerProject/Blueprint/Interface/BPI_Item.GetItem` MovedActor))
        (`/Game/AutobattlerProject/Blueprint/Core/BP_EventManager.OnGameObjectBuy` (`/Game/AutobattlerProject/Blueprint/FunctionLibraries/BPFL_Events.Get Event Manager`) MovedActor _item)
        (return true))
      (:`CastFailed`
        (return true)))
    (else
      (return false))))

(fn `UserConstructionScript`
  (`SceneComponent.SetRelativeScale3D` (`self.Box`) (`self.CollisionScale`)))