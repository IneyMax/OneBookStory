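; BP_StoreManager is the manager for the creature shop in the autobattler, filling the store's placements with random creatures.
; On BeginPlay it binds to the event manager's level-up and refresh events, then runs an initial refresh.
; A refresh clears each creature placement and puts in a new BP_Item carrying info from a random Creatures entry.
; Store level-up currently only prints a debug message.
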(event `self.ReceiveBeginPlay`
  (`|ExecutionSequence`
    (:`then_0`
      (add `/Game/AutobattlerProject/Blueprint/Core/BP_EventManager.OnStoreLevelUp` (`/Game/AutobattlerProject/Blueprint/FunctionLibraries/BPFL_Events.Get Event Manager`) (`|CreateDelegate` :!event `StoreLevelUp`))
      (add `/Game/AutobattlerProject/Blueprint/Core/BP_EventManager.OnStoreRefresh` (`/Game/AutobattlerProject/Blueprint/FunctionLibraries/BPFL_Events.Get Event Manager`) (`|CreateDelegate` :!event `StoreRefresh`)))
    (:`then_1`
      (`self.StoreRefresh`))))

(event `StoreLevelUp`
  (`KismetSystemLibrary.PrintString` "ShopLevelUp"))

(event `StoreRefresh`
  (for _array_element (`self.CreaturePlacement`)
    (`/Game/AutobattlerProject/Blueprint/Gameplay/BoardGameObjects/Placement/BP_Placement_Base.ClearPlacement` _array_element)
    (bind _returnvalue (`|GenericCreateObject` "/Game/AutobattlerProject/Blueprint/Gameplay/BoardGameObjects/BP_Item.BP_Item_C" self))
    (bind _output_get (set `self.LNewItem` _returnvalue))
    (set `Item.ItemInfo` (`self.GetRandomCreatureFromPull`) _output_get)
    (`/Game/AutobattlerProject/Blueprint/Gameplay/BoardGameObjects/Placement/BP_Placement_Base.Try Create Object in Placement` _array_element (`self.LNewItem`))))

(fn `GetRandomCreatureFromPull`
  (returns (`Item Info` :type "OBSItemInfo Structure"))
  (return (`OBSItemData.ItemInfo` (`KismetArrayLibrary.Array_Random` (`self.Creatures`)))))

(fn `UserConstructionScript`)