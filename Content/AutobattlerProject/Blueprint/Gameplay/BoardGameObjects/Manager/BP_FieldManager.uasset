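; Board field manager for the autobattler, meant to handle card drag, play, sell and return-to-hand on the placement grid.
; On BeginPlay it subscribes to event manager events and caches the player controller, but the visible handlers are empty, their logic disconnected.
; Field init and archiving are also disconnected stubs, leaving placement getters and a BP_Creature spawn helper.
; A note marks play-card handling for removal from this manager.
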(event `self.ReceiveBeginPlay`
  (`self.InitEvents`)
  (bind _asbp_player_controller_main (cast `/Game/AutobattlerProject/Blueprint/Core/BP_PlayerControllerMAin` (`GameplayStatics.GetPlayerController` 0)))
  (set `self.PlayerController` _asbp_player_controller_main))

(event `OnDrag_Event`
  (params (Card :type "Object Object Reference") (CardScreenPosition :type "Vector2D Structure")))

(event `OnMoveToHand_Event`
  (params (MoveActor :type "Actor Object Reference") (Item :type "Object Object Reference")))

(event `OnPlayCard_Event`
  (params (CreatedGameObject :type "Actor Object Reference") (Item :type "Object Object Reference"))
  ;[1 1 1] Убрать из менеджера поля!
)

(event `OnSell_Event`
  (params (SoldGameObject :type "Actor Object Reference") (Item :type "Object Object Reference")))

(fn `ArchivingField`
  (locals (LSaveItems :type "Map of Integer to Object Object Reference")))

(fn `Create GameObject At Location`
  (params (Location :type "Vector Structure") (Item :type "/Game/AutobattlerProject/Blueprint/Gameplay/BoardGameObjects/BP_Item Object Reference"))
  (returns (NewCreature :type "/Game/AutobattlerProject/Blueprint/Gameplay/BoardGameObjects/BoardGameObjects/BP_Creature Object Reference"))
  (bind _returnvalue (`|SpawnActorFromClass` "/Game/AutobattlerProject/Blueprint/Gameplay/BoardGameObjects/BoardGameObjects/BP_Creature.BP_Creature_C" (`KismetMathLibrary.MakeTransform` (`KismetMathLibrary.MakeVector` (.x Location) (.y Location) 20.0)) "Undefined" "OverrideRootScale" null null Item (`GameplayStatics.GetPlayerPawn` 0)))
  (return _returnvalue))

(fn `GetOpponentPlacement`
  (returns (OpponentPlacement :type "Array of PlacementBase Object Reference"))
  (return (`self.OpponentPlacement`)))

(fn `GetPlayerPlacement`
  (returns (PlayerPlacement :type "Array of PlacementBase Object Reference"))
  (locals (LPlayerPlacement :type "Array of PlacementBase Object Reference"))
  (return (`self.PlayerPlacement`)))

(fn `InitEvents`
  (`|ExecutionSequence`
    (:`then_0`
      (add `/Game/AutobattlerProject/Blueprint/Core/BP_EventManager.OnMoveGameObjectToHand` (`/Game/AutobattlerProject/Blueprint/FunctionLibraries/BPFL_Events.Get Event Manager`) (`|CreateDelegate` :!event `OnMoveToHand_Event`)))
    (:`then_1`
      (add `/Game/AutobattlerProject/Blueprint/Core/BP_EventManager.OnPlayCard` (`/Game/AutobattlerProject/Blueprint/FunctionLibraries/BPFL_Events.Get Event Manager`) (`|CreateDelegate` :!event `OnPlayCard_Event`)))
    (:`then_2`
      (add `/Game/AutobattlerProject/Blueprint/Core/BP_EventManager.OnDragCard` (`/Game/AutobattlerProject/Blueprint/FunctionLibraries/BPFL_Events.Get Event Manager`) (`|CreateDelegate` :!event `OnDrag_Event`)))
    (:`then_3`
      (add `/Game/AutobattlerProject/Blueprint/Core/BP_EventManager.OnSell` (`/Game/AutobattlerProject/Blueprint/FunctionLibraries/BPFL_Events.Get Event Manager`) (`|CreateDelegate` :!event `OnSell_Event`)))
    (:`then_4`
      (add `/Game/AutobattlerProject/Blueprint/Core/BP_EventManager.OnPlayCardCancel` (`/Game/AutobattlerProject/Blueprint/FunctionLibraries/BPFL_Events.Get Event Manager`) (`|CreateDelegate` :!event `OnMoveToHand_Event`)))))

(fn `InitField`
  (locals (LPlacement :type "PlacementBase Object Reference")))

(fn `UserConstructionScript`)