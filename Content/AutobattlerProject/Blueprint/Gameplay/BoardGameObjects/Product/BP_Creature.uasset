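; BP_Creature is a creature board piece for the autobattler, derived from a parent board-object class.
; Its construction script fills name, rank, health and attack texts from the Item's info and creature stats map.
; On interaction it moves into the target object's placement, or into the target if it is a placement, otherwise its default placement returns it.
; AttackTarget only prints the attacked creature's name.
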(event `AttackTarget`
  (params (AttackedCreature :type "/Game/AutobattlerProject/Blueprint/Gameplay/BoardGameObjects/Product/BP_Creature Object Reference"))
  (`KismetSystemLibrary.PrintString` (`KismetSystemLibrary.GetDisplayName` AttackedCreature)))

(fn `Interact With Object`
  (params (Object :type "Actor Object Reference"))
  (`parent.Interact With Object` Object)
  (bind _asbp_board_game_objects_base (cast `/Game/AutobattlerProject/Blueprint/Gameplay/BoardGameObjects/Product/BP_BoardGameObjectsBase` Object)
    (:`then`
      (set `self.NewPlacement` (`self.GetObjectPlacement` _asbp_board_game_objects_base))
      (`/Game/AutobattlerProject/Blueprint/Gameplay/BoardGameObjects/Placement/BP_Placement_Base.Add Creature in Placement` (`self.NewPlacement`) self :!label _label))
    (:`CastFailed`
      (bind _asbp_placement_base (cast `/Game/AutobattlerProject/Blueprint/Gameplay/BoardGameObjects/Placement/BP_Placement_Base` Object)
        (:`then`
          (set `self.NewPlacement` _asbp_placement_base)
          (goto _label))
        (:`CastFailed`
          (`/Game/AutobattlerProject/Blueprint/Gameplay/BoardGameObjects/Placement/BP_Placement_Base.ReturnActorToPlacement` (`self.DefaultPlacement`)))))))

(fn `UserConstructionScript`
  (bind _item (`self.Item`))
  (bind (_name _rank _species _fraction _creatureinfo) (break `OBSItemInfo` (`Item.ItemInfo` _item)))
  (bind (_isvalid _abilities _creaturestats) (break `CreatureInfo` _creatureinfo))
  (`parent.UserConstructionScript`)
  (if (`KismetSystemLibrary.IsValid` _item)
    (`|ExecutionSequence`
      (:`then_0`
        (`TextRenderComponent.K2_SetText` (`self.Name_Text`) (`KismetTextLibrary.Conv_NameToText` _name)))
      (:`then_1`
        (`TextRenderComponent.K2_SetText` (`self.ItemRank_Text`) (`KismetTextLibrary.Conv_IntToText` _rank)))
      (:`then_2`
        (`TextRenderComponent.K2_SetText` (`self.Health_Text`) (`KismetTextLibrary.Conv_IntToText` (`BlueprintMapLibrary.Map_Find` _creaturestats "Health"))))
      (:`then_3`
        (`TextRenderComponent.K2_SetText` (`self.Attack_Text`) (`KismetTextLibrary.Conv_IntToText` (`BlueprintMapLibrary.Map_Find` _creaturestats "Attack")))))))