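; Base actor for draggable board objects in the autobattler, with a placement reference and Buy/Sell functions that destroy it and return its item.
; StartInteract opens a Tick gate that moves the actor to the player controller's mouse world position at a fixed height.
; EndInteract passes the actor under the cursor to an empty InteractWithObject hook; CancelInteract returns the object to its placement.
; Cursor-over events are empty, and the preview card widget code never runs.
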(event `self.ReceiveBeginPlay`
  (bind _asbp_game_player_controller (cast `/Game/AutobattlerProject/Blueprint/Core/BP_GamePlayerController` (`self.GetInstigatorController`)))
  (set `self.Player Controller` _asbp_game_player_controller))

(event `self.ReceiveActorBeginCursorOver`)

(event `self.ReceiveActorEndCursorOver`)

(event `self.ReceiveTick`
  (params (DeltaSeconds :type "Float (single-precision)"))
  (`/Engine/EditorBlueprintResources/StandardMacros.Gate` true :!label _label
    (:`Exit`
      (bind _location (`/Game/AutobattlerProject/Blueprint/Core/BP_GamePlayerController.Mouse To World Space` (`self.Player Controller`) null))
      (`self.MoveToMouseLocation` _location))))

(event `/Game/AutobattlerProject/Blueprint/Interface/BPI_ObjectInteract.StartInteract`
  (params (bIsStore :type Boolean))
  (goto _label :!via `Open`))

(event `/Game/AutobattlerProject/Blueprint/Interface/BPI_ObjectInteract.CancelInteract`
  (params (bIsStore :type Boolean))
  (`/Game/AutobattlerProject/Blueprint/Gameplay/BoardGameObjects/Placement/BP_Placement_Base.ReturnActorToPlacement` (`self.DefaultPlacement`))
  (goto _label :!via `Close`))

(event `/Game/AutobattlerProject/Blueprint/Interface/BPI_ObjectInteract.EndInteract`
  (params (bIsStore :type Boolean))
  (bind (_location _hitactor) (`/Game/AutobattlerProject/Blueprint/Core/BP_GamePlayerController.Mouse To World Space` (`self.Player Controller`) self))
  (`self.Interact With Object` _hitactor)
  (goto _label :!via `Close`))

(fn `Buy`
  (returns (Item :type "/Game/AutobattlerProject/Blueprint/Gameplay/BoardGameObjects/BP_Item Object Reference"))
  (`self.K2_DestroyActor`)
  (return (`self.Item`)))

(fn `GetObjectPlacement`
  (returns (Placement :type "/Game/AutobattlerProject/Blueprint/Gameplay/BoardGameObjects/Placement/BP_Placement_Base Object Reference"))
  (return (`self.DefaultPlacement`)))

(fn `GetPlacementConfig`
  (returns (PlacementInfo :type "OBSPlacementInfo Structure"))
  (bind _placementinfo (message `/Game/AutobattlerProject/Blueprint/Interface/BPI_ObjectInteract.GetPlacementConfig` (`self.DefaultPlacement`)))
  (return _placementinfo))

(fn `Interact With Object`
  (params (Object :type "Actor Object Reference")))

(fn `MoveToMouseLocation`
  (params (MouseLocation :type "Vector Structure"))
  (`self.K2_SetActorLocation` (`KismetMathLibrary.MakeVector` (.x MouseLocation) (.y MouseLocation) 25.0)))

(fn `Sell`
  (returns (Item :type "/Game/AutobattlerProject/Blueprint/Gameplay/BoardGameObjects/BP_Item Object Reference"))
  (`self.K2_DestroyActor`)
  (return (`self.Item`)))

(fn `SetObjectPlacement`
  (params (Placement :type "/Game/AutobattlerProject/Blueprint/Gameplay/BoardGameObjects/Placement/BP_Placement_Base Object Reference"))
  (set `self.DefaultPlacement` Placement))

(fn `UserConstructionScript`)