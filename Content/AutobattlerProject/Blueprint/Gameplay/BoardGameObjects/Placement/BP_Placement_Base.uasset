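; BP_Placement_Base is a base board slot for the autobattler that holds a single game object and keeps it snapped to the slot's position at a fixed height.
; It can spawn an item-based BP_BoardGameObjectsBase into an empty slot, passing itself as default placement, or clear its occupant.
; Interacting swaps occupants with the incoming object's placement through message calls, or simply adopts the object.
; Adding an object binds its destroy event to empty the slot.
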(event `OnGameObjectDestroyed_Event` :!signature `self.OnDestroyed`
  (params (DestroyedActor :type "Actor Object Reference"))
  ;[1 1 1] TODO: Переделать событийное взаимодействие мест и объектов - управление подпиской на перемещение между местами
  (clear `self.OnDestroyed` DestroyedActor)
  (`self.Remove Object From Placement`))

(event `self.Add Object In Placement`
  (params (GameObject :type "Actor Object Reference"))
  (bind _output_get (set `self.ObjectInPlacement` GameObject))
  (`/Engine/EditorBlueprintResources/StandardMacros.IsValid` _output_get
    (:`Is Valid`
      (add `self.OnDestroyed` _output_get (`|CreateDelegate` :!event `OnGameObjectDestroyed_Event`))
      (message `/Game/AutobattlerProject/Blueprint/Interface/BPI_BoardObject.Set Object Placement` _output_get self)
      (`self.K2_SetActorLocation` _output_get (`KismetMathLibrary.MakeVector` (.x (`self.K2_GetActorLocation`)) (.y (`self.K2_GetActorLocation`)) 20.0) false false))))

(fn `CancelInteract`
  (returns (bIsReturnToDefaultState :type Boolean))
  (return false))

(fn `Check Add Object`
  (params (PlacementInfo :type "OBSPlacementInfo Structure") (Placement :type "/Game/AutobattlerProject/Blueprint/Gameplay/BoardGameObjects/Placement/BP_Placement_Base Object Reference"))
  (if (or false (== self Placement))
    (`self.Return Actor to Defult Placement` Placement)))

(fn `ClearPlacement`
  (bind _removedobject (`self.Remove Object From Placement`))
  (`/Engine/EditorBlueprintResources/StandardMacros.IsValid` _removedobject
    (:`Is Valid`
      (`self.K2_DestroyActor` _removedobject))))

(fn `Get Object From Placement`
  (returns (BoardGameObject :type "Actor Object Reference"))
  (return (`self.ObjectInPlacement`)))

(fn `Interacted`
  (params (InteractedActor :type "Actor Object Reference"))
  (returns (bIsInteracted :type Boolean))
  (bind _placement (message `/Game/AutobattlerProject/Blueprint/Interface/BPI_BoardObject.Get Object Placement` InteractedActor))
  (`/Engine/EditorBlueprintResources/StandardMacros.IsValid` _placement
    (:`Is Valid`
      (bind _boardgameobject (message `/Game/AutobattlerProject/Blueprint/Interface/BPI_Placement.Get Object From Placement` _placement))
      (bind _removedobject (`self.Remove Object From Placement`))
      (`self.Add Object In Placement` _boardgameobject)
      (message `/Game/AutobattlerProject/Blueprint/Interface/BPI_Placement.Add Object In Placement` _placement _removedobject)
      (return true))
    (:`Is Not Valid`
      (`self.Add Object In Placement` InteractedActor)
      (return true))))

(fn `Remove Object From Placement`
  (returns (RemovedObject :type "Actor Object Reference"))
  (locals (LObjectInPlacement :type "Actor Object Reference"))
  (set `local.LObjectInPlacement` (`self.ObjectInPlacement`))
  (set `self.ObjectInPlacement` null)
  (return (`local.LObjectInPlacement`)))

(fn `Return Actor to Defult Placement`
  (bind _objectinplacement (`self.ObjectInPlacement`)
    (:`then`
      (`self.K2_SetActorLocation` _objectinplacement (`KismetMathLibrary.MakeVector` (.x (`self.K2_GetActorLocation`)) (.y (`self.K2_GetActorLocation`)) 20.0) false false))
    (:`else`)))

(fn `StartInteract`
  (returns (bIsSuccess :type Boolean))
  (return true))

(fn `Try Create Object in Placement`
  (params (Item :type "/Game/AutobattlerProject/Blueprint/Gameplay/BoardGameObjects/BP_Item Object Reference"))
  (returns (bIsSuccess :type Boolean))
  (`self.ObjectInPlacement`
    (:`then`
      (return false))
    (:`else`
      (bind _returnvalue (`|SpawnActorFromClass` "/Game/AutobattlerProject/Blueprint/Gameplay/BoardGameObjects/BoardGameObjects/BP_BoardGameObjectsBase.BP_BoardGameObjectsBase_C" (`KismetMathLibrary.MakeTransform` (`KismetMathLibrary.MakeVector` (.x (.location (`self.GetTransform`))) (.y (.location (`self.GetTransform`))) 20.0) (.rotation (`self.GetTransform`))) "Undefined" "OverrideRootScale" null self Item (`GameplayStatics.GetPlayerPawn` 0)))
      (return true))))

(fn `UserConstructionScript`
  (bind _objectinplacement (`self.ObjectInPlacement`)
    (:`then`
      (`self.K2_SetActorLocation` _objectinplacement (`KismetMathLibrary.MakeVector` (.x (`self.K2_GetActorLocation`)) (.y (`self.K2_GetActorLocation`)) 20.0) false false))
    (:`else`)))