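; Shop manager for an autobattler that stocks the store's creature slots with random offers.
; On BeginPlay, ShopRefresh clears each slot in CreaturePlacement, constructs a new BP_Item with ItemInfo from a random Creatures entry, and asks the slot to create it.
; The pick is a plain random draw, with no weighting or removal from the pool.
; ShopLevelUp is a stub that only prints a string.
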(event `self.ReceiveBeginPlay`
  (`self.ShopRefresh`))

(event `ShopLevelUp`
  (`KismetSystemLibrary.PrintString` "ShopLevelUp"))

(fn `GetRandomCreatureFromPull`
  (returns (`Item Info` :type "OBSItemInfo Structure"))
  (return (`OBSItemData.ItemInfo` (`KismetArrayLibrary.Array_Random` (`self.Creatures`)))))

(fn `ShopRefresh`
  (locals (LNewItem :type "/Game/AutobattlerProject/Blueprint/Gameplay/BoardGameObjects/BP_Item Object Reference"))
  (for _array_element (`self.CreaturePlacement`)
    (`/Game/AutobattlerProject/Blueprint/Gameplay/BoardGameObjects/Placement/BP_Placement_Base.ClearPlacement` _array_element)
    (bind _returnvalue (`|GenericCreateObject` "/Game/AutobattlerProject/Blueprint/Gameplay/BoardGameObjects/BP_Item.BP_Item_C" self))
    (bind _output_get (set `local.LNewItem` _returnvalue))
    (set `Item.ItemInfo` (`self.GetRandomCreatureFromPull`) _output_get)
    (`/Game/AutobattlerProject/Blueprint/Gameplay/BoardGameObjects/Placement/BP_Placement_Base.Try Create Object in Placement` _array_element (`local.LNewItem`))))

(fn `UserConstructionScript`)