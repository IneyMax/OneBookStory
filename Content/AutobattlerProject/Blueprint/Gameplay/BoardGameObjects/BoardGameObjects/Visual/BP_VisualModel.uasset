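; BP_VisualModel is the visual representation of a board item in the autobattler, showing its mesh and stats.
; ShowItemInfo validates the Item, then writes its name, rank, and creature Health and Attack to text elements.
; SetCreatureVisual and SetWeaponVisual switch the static mesh to a flattened cube or cylinder to distinguish item types.
; The hover preview widget is an unfinished TODO: the cursor events are empty and the widget create/remove logic is disconnected.
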(event `self.ReceiveActorBeginCursorOver`
  ;[1 1 1] TODO: Preview widget
)

(event `self.ReceiveActorEndCursorOver`
  ;[1 1 1] TODO: Preview widget
)

(fn `SetCreatureVisual`
  (`StaticMeshComponent.SetStaticMesh` (`self.StaticMesh`) (`self.CubeMesh`))
  (`SceneComponent.SetRelativeScale3D` (`self.StaticMesh`) (1.0 1.0 0.1)))

(fn `SetWeaponVisual`
  (`StaticMeshComponent.SetStaticMesh` (`self.StaticMesh`) (`self.CylinderMesh`))
  (`SceneComponent.SetRelativeScale3D` (`self.StaticMesh`) (1.0 1.0 0.1)))

(fn `ShowItemInfo`
  (bind _item (`self.Item`))
  (bind (_name _rank _species _fraction _creatureinfo) (break `OBSItemInfo` (`Item.ItemInfo` _item)))
  (bind (_isvalid _abilities _creaturestats) (break `CreatureInfo` _creatureinfo))
  (if (`KismetSystemLibrary.IsValid` _item)
    (`|ExecutionSequence`
      (:`then_0`
        (`TextRenderComponent.K2_SetText` (`self.Name_Text`) (`KismetTextLibrary.Conv_NameToText` _name)))
      (:`then_1`
        (`TextRenderComponent.K2_SetText` (`self.ItemRank_Text`) (`KismetTextLibrary.Conv_IntToText` _rank)))
      (:`then_2`
        (`TextRenderComponent.K2_SetText` (`self.Health_Text`) (`KismetTextLibrary.Conv_IntToText` (`BlueprintMapLibrary.Map_Find` _creaturestats "Health"))))
      (:`then_3`
        (`TextRenderComponent.K2_SetText` (`self.Attack_Text`) (`KismetTextLibrary.Conv_IntToText` (`BlueprintMapLibrary.Map_Find` _creaturestats "Attack")))))))

(fn `UserConstructionScript`)