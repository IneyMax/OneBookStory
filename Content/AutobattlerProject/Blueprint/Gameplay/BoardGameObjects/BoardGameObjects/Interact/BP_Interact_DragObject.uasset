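; BP_Interact_DragObject is an interaction strategy for dragging a board game object and playing it as a creature or weapon.
; DragStart binds EventManager events so the owner follows the mouse and switches Weapon or Creature visuals by what is detected.
; Dropping on an empty placement adds the owner, swaps its strategy to BP_Interact_Creature and fires OnCardPlay.
; Interacting with a game object instead adds the owner as its weapon and attaches it.
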(event `self.UpdateBegin`
  (add `/Game/AutobattlerProject/Blueprint/EventManagers/BP_PlayerInteractEventManager.OnMouseLocationUpdate` (`self.EventManager`) (`|CreateDelegate` :!event `Update`))
  (add `/Game/AutobattlerProject/Blueprint/EventManagers/BP_PlayerInteractEventManager.OnBoardGameObjectDetected` (`self.EventManager`) (`|CreateDelegate` :!event `SwitchVisualModel`)))

(event `self.UpdateEnd`
  (remove `/Game/AutobattlerProject/Blueprint/EventManagers/BP_PlayerInteractEventManager.OnMouseLocationUpdate` (`self.EventManager`) (`|CreateDelegate` :!event `Update`))
  (remove `/Game/AutobattlerProject/Blueprint/EventManagers/BP_PlayerInteractEventManager.OnBoardGameObjectDetected` (`self.EventManager`) (`|CreateDelegate` :!event `SwitchVisualModel`)))

(event `self.Update`
  (params (MouseLocation :type "Vector Structure"))
  (`Actor.K2_SetActorLocation` (`self.Owner`) (`KismetMathLibrary.MakeVector` (.x MouseLocation) (.y MouseLocation) 25.0) false false))

(event `SwitchVisualModel`
  (params (Placement :type "Actor Object Reference"))
  (cast `/Game/AutobattlerProject/Blueprint/Gameplay/BoardGameObjects/BoardGameObjects/BP_BoardGameObjectsBase` Placement
    (:`then`
      (message `/Game/AutobattlerProject/Blueprint/Interface/BPI_BoardObject.SwitchGameObjectState` (`self.Owner`) "Weapon"))
    (:`CastFailed`
      (message `/Game/AutobattlerProject/Blueprint/Interface/BPI_BoardObject.SwitchGameObjectState` (`self.Owner`) "Creature"))))

(event `OnDestroyed_Event`
  (params (DestroyedActor :type "Actor Object Reference"))
  (`self.UpdateEnd`)
  (set `self.Owner` null))

(event `self.SetOwnerGameObject`
  (params (NewOwner :type "/Game/AutobattlerProject/Blueprint/Gameplay/BoardGameObjects/BoardGameObjects/BP_BoardGameObjectsBase Object Reference"))
  (bind _output_get (set `self.Owner` NewOwner))
  (add `Actor.OnDestroyed` _output_get (`|CreateDelegate` :!event `OnDestroyed_Event`)))

(fn `CancelInteract`
  (params (PastPlacement :type "Actor Object Reference"))
  (returns (bIsReturnToDefaultState :type Boolean))
  (`self.UpdateEnd`)
  (return false))

(fn `DragEnd`
  (returns (bIsSuccess :type Boolean))
  (return true))

(fn `DragStart`
  (returns (bIsSuccess :type Boolean))
  (`self.UpdateBegin`)
  (return true))

(fn `InteractWithGameObject`
  (params (InteractedActor :type "Actor Object Reference"))
  (returns (bIsInteracted :type Boolean))
  (bind _asbp_board_game_objects_base (cast `/Game/AutobattlerProject/Blueprint/Gameplay/BoardGameObjects/BoardGameObjects/BP_BoardGameObjectsBase` (`self.Owner`))
    (:`then`
      (message `/Game/AutobattlerProject/Blueprint/Interface/BPI_BoardObject.AddWeaponToPossession` InteractedActor _asbp_board_game_objects_base)
      (`Actor.K2_AttachToActor` (`self.Owner`) InteractedActor "None" "KeepRelative" "KeepRelative" "KeepRelative" true)
      (return true))
    (:`CastFailed`
      (return false))))

(fn `InteractWithPlacement`
  (params (PastPlacement :type "Actor Object Reference") (NewPlacement :type "Actor Object Reference"))
  (returns (bIsInteracted :type Boolean))
  (bind _owner (`self.Owner`))
  (bind _boardgameobject (message `/Game/AutobattlerProject/Blueprint/Interface/BPI_Placement.Get Object From Placement` NewPlacement))
  (`/Engine/EditorBlueprintResources/StandardMacros.IsValid` _boardgameobject
    (:`Is Valid`
      (return false))
    (:`Is Not Valid`
      (bind _bissuccess (message `/Game/AutobattlerProject/Blueprint/Interface/BPI_Placement.Add Object In Placement` NewPlacement (`self.Owner`)))
      ;[1 1 1] TODO
      (bind _returnvalue (`|GenericCreateObject` "/Game/AutobattlerProject/Blueprint/Gameplay/BoardGameObjects/BoardGameObjects/Interact/BP_Interact_Creature.BP_Interact_Creature_C" _owner _owner (`self.EventManager`)))
      (message `/Game/AutobattlerProject/Blueprint/Interface/BPI_BoardObject.Set Interact Strategy` (`self.Owner`) _returnvalue)
      (bind _item (message `/Game/AutobattlerProject/Blueprint/Interface/BPI_Item.GetItem` (`self.Owner`)))
      (`/Game/AutobattlerProject/Blueprint/EventManagers/BP_PlayerInteractEventManager.OnCardPlay` (`self.EventManager`) (`self.Owner`) _item)
      (return _bissuccess))))