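; Interaction handler for creature board objects in the autobattler, covering dragging, placement and cleanup on destruction.
; While dragging, it subscribes to EventManager mouse-location updates and moves the owner at a fixed height.
; Dropping on a valid placement swaps both placements' occupants; cancelling returns the creature to its default placement, and interacting with another object is refused.
; When the owner is destroyed, its possessed weapons are returned to the hand through EventManager.
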(event `self.UpdateBegin`
  (add `/Game/AutobattlerProject/Blueprint/Core/BP_EventManager.OnMouseLocationUpdate` (`self.EventManager`) (`|CreateDelegate` :!event `Update`)))

(event `self.UpdateEnd`
  (remove `/Game/AutobattlerProject/Blueprint/Core/BP_EventManager.OnMouseLocationUpdate` (`self.EventManager`) (`|CreateDelegate` :!event `Update`)))

(event `self.Update`
  (params (MouseLocation :type "Vector Structure"))
  (`Actor.K2_SetActorLocation` (`self.Owner`) (`KismetMathLibrary.MakeVector` (.x MouseLocation) (.y MouseLocation) 25.0) false false))

(event `OnDestroyed_Event`
  (params (DestroyedActor :type "Actor Object Reference"))
  (`self.UpdateEnd`)
  (set `self.Owner` null)
  (bind _weaponspossession (message `/Game/AutobattlerProject/Blueprint/Interface/BPI_BoardObject.GetWeaponsPossession` DestroyedActor))
  (for _array_element _weaponspossession
    (bind _item (message `/Game/AutobattlerProject/Blueprint/Interface/BPI_Item.GetItem` _array_element))
    (`/Game/AutobattlerProject/Blueprint/Core/BP_EventManager.OnGameObjectReturnToHand` (`self.EventManager`) _array_element _item)))

(event `self.SetOwnerGameObject`
  (params (NewOwner :type "/Game/AutobattlerProject/Blueprint/Gameplay/BoardGameObjects/BoardGameObjects/BP_BoardGameObjectsBase Object Reference"))
  (bind _output_get (set `self.Owner` NewOwner))
  (add `Actor.OnDestroyed` _output_get (`|CreateDelegate` :!event `OnDestroyed_Event`)))

(fn `CancelInteract`
  (params (PastPlacement :type "Actor Object Reference"))
  (returns (bIsReturnToDefaultState :type Boolean))
  (`self.UpdateEnd`)
  (bind _bisreturned (message `/Game/AutobattlerProject/Blueprint/Interface/BPI_Placement.Return Actor To Defult Placement` PastPlacement))
  (return _bisreturned))

(fn `DragEnd`
  (returns (bIsSuccess :type Boolean))
  (return true))

(fn `DragStart`
  (returns (bIsSuccess :type Boolean))
  (`self.UpdateBegin`)
  (return true))

(fn `InteractWithGameObject`
  (params (InteractedActor :type "Actor Object Reference"))
  (returns (bIsInteracted :type Boolean))
  (`self.UpdateEnd`)
  (return false))

(fn `InteractWithPlacement`
  (params (PastPlacement :type "Actor Object Reference") (NewPlacement :type "Actor Object Reference"))
  (returns (bIsInteracted :type Boolean))
  (`/Engine/EditorBlueprintResources/StandardMacros.IsValid` NewPlacement
    (:`Is Valid`
      (bind _removedobject (message `/Game/AutobattlerProject/Blueprint/Interface/BPI_Placement.Remove Object from Placement` NewPlacement))
      (bind _removedobject_2 (message `/Game/AutobattlerProject/Blueprint/Interface/BPI_Placement.Remove Object from Placement` PastPlacement))
      (message `/Game/AutobattlerProject/Blueprint/Interface/BPI_Placement.Add Object In Placement` NewPlacement _removedobject_2)
      (message `/Game/AutobattlerProject/Blueprint/Interface/BPI_Placement.Add Object In Placement` PastPlacement _removedobject)
      (return true))
    (:`Is Not Valid`
      (return false))))