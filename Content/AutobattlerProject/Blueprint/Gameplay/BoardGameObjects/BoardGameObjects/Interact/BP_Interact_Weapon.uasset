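; BP_Interact_Weapon is an interaction object for weapons on the board, moving its owning actor with the mouse.
; UpdateBegin and UpdateEnd bind and unbind the EventManager's mouse-location event, while Update places the owner at the mouse X/Y at a fixed height.
; Start, end, cancel, game-object and placement interactions are stubs that return false, so only the follow behavior is implemented.
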(event `/Game/AutobattlerProject/Blueprint/Interface/BPI_Interact.SetOwner`
  (params (NewOwner :type "Actor Object Reference"))
  (set `self.Owner` NewOwner))

(event `/Game/AutobattlerProject/Blueprint/Interface/BPI_Interact.UpdateBegin`
  (add `/Game/AutobattlerProject/Blueprint/Core/BP_EventManager.OnMouseLocationUpdate` (`self.EventManager`) (`|CreateDelegate` :!event `Update`)))

(event `/Game/AutobattlerProject/Blueprint/Interface/BPI_Interact.UpdateEnd`
  (remove `/Game/AutobattlerProject/Blueprint/Core/BP_EventManager.OnMouseLocationUpdate` (`self.EventManager`) (`|CreateDelegate` :!event `Update`)))

(event `/Game/AutobattlerProject/Blueprint/Interface/BPI_Interact.Update`
  (params (MouseLocation :type "Vector Structure"))
  (`Actor.K2_SetActorLocation` (`self.Owner`) (`KismetMathLibrary.MakeVector` (.x MouseLocation) (.y MouseLocation) 25.0) false false))

(fn `CancelInteract`
  (returns (bIsReturnToDefaultState :type Boolean))
  (return false))

(fn `EndInteract`
  (returns (bIsSuccess :type Boolean))
  (return false))

(fn `InteractWithGameObject`
  (params (InteractedActor :type "Actor Object Reference"))
  (returns (bIsInteracted :type Boolean))
  (return false))

(fn `InteractWithPlacement`
  (params (Placement :type "Actor Object Reference"))
  (returns (bIsInteracted :type Boolean))
  (return false))

(fn `StartInteract`
  (returns (bIsSuccess :type Boolean))
  (return false))