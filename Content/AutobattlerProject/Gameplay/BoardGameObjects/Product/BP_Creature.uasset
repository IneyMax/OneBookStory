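; BP_Creature is a creature board game object for the autobattler that can be assigned to placements.
; Interacting with another board object resolves that object's placement, while interacting with a placement uses it directly, and the creature then adds itself there.
; Any other target makes its default placement return the actor.
; The AttackTarget event only prints the attacked creature's name.
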(event `AttackTarget`
  (params (AttackedCreature :type "/Game/AutobattlerProject/Gameplay/BoardGameObjects/Product/BP_Creature Object Reference"))
  (`KismetSystemLibrary.PrintString` (`KismetSystemLibrary.GetDisplayName` AttackedCreature)))

(fn `Interact With Object`
  (params (Object :type "Actor Object Reference"))
  (`parent.Interact With Object` Object)
  (bind _asbp_board_game_objects_base (cast `/Game/AutobattlerProject/Gameplay/BoardGameObjects/Product/BP_BoardGameObjectsBase` Object)
    (:`then`
      (set `self.NewPlacement` (`self.GetObjectPlacement` _asbp_board_game_objects_base))
      (`/Game/AutobattlerProject/Gameplay/BoardGameObjects/Placement/BP_Placement_Base.Add Creature in Placement` (`self.NewPlacement`) self :!label _label))
    (:`CastFailed`
      (bind _asbp_placement_base (cast `/Game/AutobattlerProject/Gameplay/BoardGameObjects/Placement/BP_Placement_Base` Object)
        (:`then`
          (set `self.NewPlacement` _asbp_placement_base)
          (goto _label))
        (:`CastFailed`
          (`/Game/AutobattlerProject/Gameplay/BoardGameObjects/Placement/BP_Placement_Base.ReturnActorToPlacement` (`self.DefaultPlacement`)))))))

(fn `UserConstructionScript`
  (`parent.UserConstructionScript`))