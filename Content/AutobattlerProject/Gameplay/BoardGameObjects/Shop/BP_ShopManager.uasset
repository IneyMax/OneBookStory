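; BP_ShopManager runs the autobattler shop, filling its creature placements with creatures on offer.
; On BeginPlay and on ShopRefresh, it loops over CreaturePlacement and asks each slot to create an object from a randomly picked creature.
; GetRandomCreatureFromPull returns a uniformly random entry from the Creatures array.
; ShopLevelUp is a stub that only prints a debug string.
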(event `self.ReceiveBeginPlay`
  (for _array_element (`self.CreaturePlacement`)
    (`/Game/AutobattlerProject/Gameplay/BoardGameObjects/Placement/BP_Placement_Base.Try Create Object in Placement` _array_element (`self.GetRandomCreatureFromPull`))))

(event `ShopLevelUp`
  (`KismetSystemLibrary.PrintString` "ShopLevelUp"))

(event `ShopRefresh`
  (for _array_element (`self.CreaturePlacement`)
    (`/Game/AutobattlerProject/Gameplay/BoardGameObjects/Placement/BP_Placement_Base.Try Create Object in Placement` _array_element (`self.GetRandomCreatureFromPull`))))

(fn `GetRandomCreatureFromPull`
  (returns (Payload :type "OBSItemCreature Object Reference"))
  (return (`KismetArrayLibrary.Array_Random` (`self.Creatures`))))

(fn `UserConstructionScript`)