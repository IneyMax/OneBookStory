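; Base board slot actor for the autobattler that holds a single object, such as a creature.
; Spawns a BP_Creature from item info when empty, and handles adding, removing and swapping objects between slots.
; Adding an object sets its placement back-reference and snaps it to the slot's XY at a fixed height, also reapplied on BeginPlay and return.
; CheckAddObject only handles same-slot returns, and GetPlacementConfig is empty.
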(event `self.ReceiveBeginPlay`
  (bind _objectinplacement (`self.ObjectInPlacement`)
    (:`then`
      (`self.K2_SetActorLocation` _objectinplacement (`KismetMathLibrary.MakeVector` (.x (`self.K2_GetActorLocation`)) (.y (`self.K2_GetActorLocation`)) 20.0) false false))
    (:`else`)))

(fn `Add Creature in Placement`
  (params (ObjectAdded :type "/Game/AutobattlerProject/Gameplay/BoardGameObjects/Product/BP_BoardGameObjectsBase Object Reference"))
  (`self.Add Object in Placement` (`/Game/AutobattlerProject/Gameplay/BoardGameObjects/Product/BP_BoardGameObjectsBase.GetObjectPlacement` ObjectAdded) (`self.ObjectInPlacement`))
  (`self.Add Object in Placement` ObjectAdded))

(fn `Add Object in Placement`
  (params (ObjectAdded :type "/Game/AutobattlerProject/Gameplay/BoardGameObjects/Product/BP_BoardGameObjectsBase Object Reference"))
  (bind _output_get (set `self.ObjectInPlacement` ObjectAdded))
  (`/Engine/EditorBlueprintResources/StandardMacros.IsValid` _output_get
    (:`Is Valid`
      (`/Game/AutobattlerProject/Gameplay/BoardGameObjects/Product/BP_BoardGameObjectsBase.SetObjectPlacement` _output_get self)
      (`self.K2_SetActorLocation` _output_get (`KismetMathLibrary.MakeVector` (.x (`self.K2_GetActorLocation`)) (.y (`self.K2_GetActorLocation`)) 20.0) false false))))

(fn `Check Add Object`
  (params (PlacementInfo :type "OBSPlacementInfo Structure") (Placement :type "/Game/AutobattlerProject/Gameplay/BoardGameObjects/Placement/BP_Placement_Base Object Reference"))
  (if (or false (== self Placement))
    (`self.ReturnActorToPlacement` Placement)))

(fn `Get Object from Placement`
  (returns (ObjectInPlacement :type "/Game/AutobattlerProject/Gameplay/BoardGameObjects/Product/BP_BoardGameObjectsBase Object Reference"))
  (return (`self.ObjectInPlacement`)))

(fn `GetPlacementConfig`
  (returns (PlacementInfo :type "OBSPlacementInfo Structure"))
  (return))

(fn `RemoveObjectfromPlacement`
  (returns (RemovedObject :type "/Game/AutobattlerProject/Gameplay/BoardGameObjects/Product/BP_BoardGameObjectsBase Object Reference"))
  (locals (LObjectInPlacement :type "/Game/AutobattlerProject/Gameplay/BoardGameObjects/Product/BP_BoardGameObjectsBase Object Reference"))
  (set `local.LObjectInPlacement` (`self.ObjectInPlacement`))
  (set `self.ObjectInPlacement` null)
  (return (`local.LObjectInPlacement`)))

(fn `ReturnActorToPlacement`
  (bind _objectinplacement (`self.ObjectInPlacement`)
    (:`then`
      (`self.K2_SetActorLocation` _objectinplacement (`KismetMathLibrary.MakeVector` (.x (`self.K2_GetActorLocation`)) (.y (`self.K2_GetActorLocation`)) 20.0) false false))
    (:`else`)))

(fn `SwitchObjectInPlacements`
  (params (FromPlacement :type "/Game/AutobattlerProject/Gameplay/BoardGameObjects/Placement/BP_Placement_Base Object Reference"))
  (locals (LRemovedObject :type "/Game/AutobattlerProject/Gameplay/BoardGameObjects/Product/BP_BoardGameObjectsBase Object Reference"))
  (bind _removedobject (`self.RemoveObjectfromPlacement`))
  (set `local.LRemovedObject` _removedobject)
  (bind _removedobject_2 (`self.RemoveObjectfromPlacement` FromPlacement))
  (`self.Add Object in Placement` _removedobject_2)
  (`self.Add Object in Placement` FromPlacement (`local.LRemovedObject`)))

(fn `Try Create Object in Placement`
  (params (`Item Info` :type "OBSItemInfo Structure"))
  (returns (bIsSuccess :type Boolean))
  (`self.ObjectInPlacement`
    (:`then`
      (return false))
    (:`else`
      (bind _returnvalue (`|SpawnActorFromClass` "/Game/AutobattlerProject/Gameplay/BoardGameObjects/Product/BP_Creature.BP_Creature_C" (`KismetMathLibrary.MakeTransform` (`KismetMathLibrary.MakeVector` (.x (.location (`self.GetTransform`))) (.y (.location (`self.GetTransform`))) 20.0) (.rotation (`self.GetTransform`))) "Undefined" "OverrideRootScale" null `Item Info` self (`GameplayStatics.GetPlayerPawn` 0)))
      (`self.Add Object in Placement` _returnvalue)
      (return true))))

(fn `UserConstructionScript`
  (bind _objectinplacement (`self.ObjectInPlacement`)
    (:`then`
      (`self.K2_SetActorLocation` _objectinplacement (`self.K2_GetActorLocation`) false false))
    (:`else`)))