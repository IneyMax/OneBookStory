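; BP_Placement is a placement slot actor in the autobattler that holds one object and snaps it to its own position.
; AddObjectInPlacement stores a valid object and moves it to the slot's XY at a fixed height, and a getter returns the held object.
; The construction script and BeginPlay re-snap any assigned object to the slot's full location.
; PlacementInteract returns a constant enum value.
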(event `self.ReceiveBeginPlay`
  (bind _objectinplacement (`self.ObjectInPlacement`)
    (:`then`
      (`self.K2_SetActorLocation` _objectinplacement (`self.K2_GetActorLocation`) false false))
    (:`else`)))

(fn `AddObjectInPlacement`
  (params (ObjectInPlacement :type "/Game/AutobattlerProject/Core/BP_BoardGameObjectsBase Object Reference"))
  (`/Engine/EditorBlueprintResources/StandardMacros.IsValid` ObjectInPlacement
    (:`Is Valid`
      (bind _output_get (set `self.ObjectInPlacement` ObjectInPlacement))
      (`self.K2_SetActorLocation` _output_get (`KismetMathLibrary.MakeVector` (.x (`self.K2_GetActorLocation`)) (.y (`self.K2_GetActorLocation`)) 20.0) false false))))

(fn `Get Object from Placement`
  (returns (ObjectInPlacement :type "/Game/AutobattlerProject/Core/BP_BoardGameObjectsBase Object Reference"))
  (return (`self.ObjectInPlacement`)))

(fn `PlacementInteract`
  (returns (ObjectType :type "/Game/AutobattlerProject/Enums/EBoardObjectType Enum"))
  (return "NewEnumerator1"))

(fn `UserConstructionScript`
  (bind _objectinplacement (`self.ObjectInPlacement`)
    (:`then`
      (`self.K2_SetActorLocation` _objectinplacement (`self.K2_GetActorLocation`) false false))
    (:`else`)))