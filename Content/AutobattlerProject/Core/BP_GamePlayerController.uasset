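; Player controller for an autobattler that creates the HUD and handles dragging board objects between press and release.
; Each tick, mouse or touch line traces find the hit actor and store zone, and move the held object.
; Press takes an object from a BP_Placement.
; Release over the store sells it for balance, over a placement destroys it and fires OnAddCard, and over other actors returns it to its previous placement.
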(event `self.ReceiveBeginPlay`
  (`|ExecutionSequence`
    (:`then_1`
      (bind _returnvalue (`|CreateWidget` "/Game/AutobattlerProject/UI/WBP_HUD.WBP_HUD_C"))
      (bind _output_get (set `self.WBP_Balance` _returnvalue))
      (`UserWidget.AddToViewport` _output_get 0))))

(event `self.ReceiveTick`
  (params (DeltaSeconds :type "Float (single-precision)"))
  (set `self.bIsStore` (`self.StoreDetected`))
  (bind (_hitactor _location) (`self.Mouse to World Location`))
  (bind _output_get (set `self.Hit Actor` _hitactor))
  (bind _takenboardobject (`self.TakenBoardObject`)
    (:`then`
      (`self.K2_SetActorLocation` _takenboardobject (`KismetMathLibrary.MakeVector` (.x _location) (.y _location) (.z (`self.K2_GetActorLocation` (`self.TakenBoardObject`)))) false false))
    (:`else`)))

(event `Key|LeftMouseButton`
  (params (Key :type "Key Structure"))
  (:`Pressed`
    (bind _hit_actor (`self.Hit Actor`)
      (:`then`
        (bind _asbp_placement (cast `/Game/AutobattlerProject/Core/BP_Placement` _hit_actor))
        (set `self.PastPlacement` _asbp_placement)
        (bind _objectinplacement (`/Game/AutobattlerProject/Core/BP_Placement.Get Object from Placement` _asbp_placement))
        (set `self.TakenBoardObject` _objectinplacement))
      (:`else`)))
  (:`Released`
    (if (`self.bIsStore`)
      (bind _takenboardobject (`self.TakenBoardObject`)
        (:`then`
          (`self.K2_DestroyActor` _takenboardobject)
          (`self.ChangeBalance`))
        (:`else`))
      (else
        (bind _hit_actor_2 (`self.Hit Actor`)
          (:`then`
            (cast `/Game/AutobattlerProject/Core/BP_Placement` _hit_actor_2
              (:`then`
                (bind _takenboardobject_2 (`self.TakenBoardObject`)
                  (:`then`
                    (`self.K2_DestroyActor` _takenboardobject_2)
                    (`self.OnAddCard`))
                  (:`else`)))
              (:`CastFailed`
                (`/Game/AutobattlerProject/Core/BP_Placement.AddObjectInPlacement` (`self.PastPlacement`) (`self.TakenBoardObject`))))
            (set `self.TakenBoardObject` null))
          (:`else`))))))

(fn `ChangeBalance`
  (locals (OldBalance :type Integer :default 0))
  (bind _output_get (set `local.OldBalance` (`self.PlayerBalance`)))
  (bind _output_get_2 (set `self.PlayerBalance` (+ _output_get 3)))
  (`self.OnChangeBalance` _output_get_2 (`local.OldBalance`)))

(fn `Get World Rotation for Player`
  (params (OverrideRotationAxis :type "Rotator Structure"))
  (returns (ReturnRotation :type "Rotator Structure") (CameraValid :type Boolean))
  (bind _roll (.roll OverrideRotationAxis))
  (bind _pitch (.pitch OverrideRotationAxis))
  (bind _yaw (.yaw OverrideRotationAxis))
  (bind _returnvalue (`GameplayStatics.GetPlayerCameraManager` 0))
  (bind (_returnvalue_roll _returnvalue_pitch _returnvalue_yaw) (`KismetMathLibrary.BreakRotator` (`self.K2_GetActorRotation` _returnvalue)))
  (`/Engine/EditorBlueprintResources/StandardMacros.IsValid` _returnvalue
    (:`Is Valid`
      (return (`KismetMathLibrary.MakeRotator` (select `bool` (> _roll 0.0) :`true` _roll) (select `bool` (> _pitch 0.0) :`true` _pitch) (select `bool` (> _yaw 0.0) :`false` _returnvalue_yaw :`true` _yaw)) true))
    (:`Is Not Valid`
      (return (struct) false))))

(fn `Mouse Distance in World Space`
  (returns (Location :type "Vector Structure") (`Spawn Tranfrom` :type "Transform Structure"))
  (bind (_worldlocation _worlddirection) (`self.DeprojectMousePositionToWorld`))
  (bind _returnvalue (+ _worldlocation (* _worlddirection (`self.Distance`))))
  (return _returnvalue (`KismetMathLibrary.MakeTransform` _returnvalue (`self.Get World Rotation for Player` (struct)))))

(fn `Mouse to World Location`
  (returns (HitActor :type "Actor Object Reference") (Location :type "Vector Structure"))
  (locals (WorldLocation :type "Vector Structure") (WorldDirection :type "Vector Structure"))
  (bind (_locationx _locationy) (`self.GetInputTouchState` "Touch1"))
  (bind (_worldlocation _worlddirection) (`self.DeprojectMousePositionToWorld`))
  (bind _worldlocation_2 (`local.WorldLocation`))
  (bind (_worldposition _worlddirection_2) (`GameplayStatics.DeprojectScreenToWorld` null (`KismetMathLibrary.MakeVector2D` _locationx _locationy)))
  (if (`self.bIsMobile`)
    (set `local.WorldLocation` _worldposition) ; Mobile World Location
    (set `local.WorldDirection` _worlddirection_2) ; Moble World Direction
    (else
      (set `local.WorldLocation` _worldlocation)
      (set `local.WorldDirection` _worlddirection)))
  (bind _outhit (`KismetSystemLibrary.LineTraceSingleForObjects` :`Start` _worldlocation_2 :`End` (+ _worldlocation_2 (* (`local.WorldDirection`) 1000.0)) :`ObjectTypes` (`|MakeArray` "ObjectTypeQuery7" "ObjectTypeQuery1" :!type "EObjectTypeQuery Enum") :`DrawDebugType` "Persistent" :`DrawTime` 10.0))
  (bind (_bblockinghit _binitialoverlap _time _distance _location _impactpoint _normal _impactnormal _physmat _hitactor) (`GameplayStatics.BreakHitResult` _outhit))
  (`KismetSystemLibrary.PrintString` (`KismetStringLibrary.Conv_VectorToString` _location) true true (struct :`G` 0.66 :`B` 1.0 :`A` 1.0) 0.0)
  (return _hitactor _location))

(fn `Screen Position In World Space`
  (params (`Screen Position` :type "Vector2D Structure"))
  (returns (Location :type "Vector Structure") (`Spawn Tranfrom` :type "Transform Structure"))
  (bind (_worldposition _worlddirection) (`GameplayStatics.DeprojectScreenToWorld` self (* `Screen Position` (`WidgetLayoutLibrary.GetViewportScale`))))
  (bind _returnvalue (+ _worldposition (* _worlddirection (`self.Distance`))))
  (return _returnvalue (`KismetMathLibrary.MakeTransform` _returnvalue (`self.Get World Rotation for Player` (struct)))))

(fn `StoreDetected`
  (returns (bIsStore :type Boolean))
  (locals (WorldLocation :type "Vector Structure") (WorldDirection :type "Vector Structure"))
  (bind (_locationx _locationy) (`self.GetInputTouchState` "Touch1"))
  (bind (_worldlocation _worlddirection) (`self.DeprojectMousePositionToWorld`))
  (bind _worldlocation_2 (`local.WorldLocation`))
  (bind (_worldposition _worlddirection_2) (`GameplayStatics.DeprojectScreenToWorld` null (`KismetMathLibrary.MakeVector2D` _locationx _locationy)))
  (if (`self.bIsMobile`)
    (set `local.WorldLocation` _worldposition) ; Mobile World Location
    (set `local.WorldDirection` _worlddirection_2) ; Moble World Direction
    (else
      (set `local.WorldLocation` _worldlocation)
      (set `local.WorldDirection` _worlddirection)))
  (bind (_outhit _returnvalue) (`KismetSystemLibrary.LineTraceSingleForObjects` :`Start` _worldlocation_2 :`End` (+ _worldlocation_2 (* (`local.WorldDirection`) 1000.0)) :`ObjectTypes` (`|MakeArray` "ObjectTypeQuery8" :!type "EObjectTypeQuery Enum") :`DrawTime` 10.0))
  (`KismetSystemLibrary.PrintString` (`KismetSystemLibrary.GetDisplayName` (`.HitActor` (`GameplayStatics.BreakHitResult` _outhit))) true true (struct :`G` 1.0 :`B` 0.214649 :`A` 1.0) 0.0)
  (return _returnvalue))

(fn `UserConstructionScript`)